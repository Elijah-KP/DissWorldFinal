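; Base editor tool actor that bakes its DynamicMeshComponent into a static mesh asset using Geometry Script.
; GenerateNewStaticMesh creates a uniquely named asset in the editable folder path, based on the actor's display name, with complex-as-simple collision, and stores the reference.
; UpdateStaticMesh copies the current dynamic mesh into that stored asset.
; Both events then apply the component's materials to the static mesh.
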(event `GenerateNewStaticMesh`
  ;[1 1 1] Generate new static mesh. Uses the instance editable asset path variable as the location of the asset
  (bind _returnvalue (`BaseDynamicMeshComponent.GetDynamicMesh` (`self.DynamicMeshComponent`)))
  (bind _uniqueassetpathandname (`GeometryScriptLibrary_CreateNewAssetFunctions.CreateUniqueNewAssetPathName` (`self.Asset Folder Path`) (`KismetSystemLibrary.GetDisplayName` self) (struct) null)
    (:`Success`
      (bind _returnvalue_2 (`GeometryScriptLibrary_CreateNewAssetFunctions.CreateNewStaticMeshAssetFromMesh` _returnvalue _uniqueassetpathandname (make `GeometryScriptCreateNewStaticMeshAssetOptions` false false false (struct :`PositionPrecision` -2147483648 :`KeepPercentTriangles` 1.0 :`FallbackPercentTriangles` 1.0 :`FallbackRelativeError` 1.0) 0.0 true "CTF_UseComplexAsSimple") null)
        (:`Success`
          (bind _output_get (set `self.Static Mesh Asset` _returnvalue_2))
          (for (_array_element _array_index) (`MeshComponent.GetMaterials` (`self.DynamicMeshComponent`))
            (`StaticMesh.SetMaterial` _output_get _array_index _array_element)))))))

(event `UpdateStaticMesh`
  ;[1 1 1] Update static mesh
  (bind _returnvalue (`BaseDynamicMeshComponent.GetDynamicMesh` (`self.DynamicMeshComponent`)))
  (`GeometryScriptLibrary_StaticMeshFunctions.CopyMeshToStaticMesh` _returnvalue (`self.Static Mesh Asset`) (struct) (struct) null
    (:`Success`
      (for (_array_element _array_index) (`MeshComponent.GetMaterials` (`self.DynamicMeshComponent`))
        (`StaticMesh.SetMaterial` (`self.Static Mesh Asset`) _array_index _array_element)))))

(fn `UserConstructionScript`)